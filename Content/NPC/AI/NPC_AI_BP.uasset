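; NPC AI controller that starts a patrol behavior for its controlled pawn.
; On BeginPlay it sets up the PatrolData blackboard and runs the Patrol behavior tree.
; AI Perception target updates only print debug text naming the pawn, the sense behind the stimulus and the perceived actor, without writing to the blackboard.
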(event OnTargetPerceptionUpdated(AIPerception)
  (params (Actor :type Actor%20Object%20Reference) (Stimulus :type AI%20Stimulus%20Structure))
  (bind _returnvalue (Class|AIPerceptionSystem|GetSenseClassforStimulus Stimulus))
  (Development|PrintText (Utilities|Text|FormatText "{me}  {stimulusName}  {otherPlayer}" (Utilities|Text|ToText(String) (Utilities|GetDisplayName (Pawn|GetControlledPawn))) (Utilities|Text|ToText(String) (Utilities|GetClassDisplayName _returnvalue)) (Utilities|Text|ToText(String) (Utilities|GetObjectName Actor)))))

(event EventBeginPlay
  (Class|AIController|UseBlackboard "/Game/NPC/AI/PatrolData.PatrolData")
  (AI|RunBehaviorTree "/Game/NPC/AI/Patrol.Patrol"))

(event EventTick
  (params (DeltaSeconds :type Float%20%28single-precision%29)))

(fn ConstructionScript)
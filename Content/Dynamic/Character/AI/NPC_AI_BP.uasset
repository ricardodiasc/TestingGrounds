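; NPC AI controller that drives a guard through the GuardBehaviour behavior tree using the PatrolData blackboard.
; On BeginPlay it sets up and caches the blackboard and starts the tree.
; AI perception updates write the perceived actor to EnemyKey if it has the Enemy tag or was successfully sensed.
; Nothing here clears that key, and Enemy-tagged actors are written even when sensing fails.
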(event OnTargetPerceptionUpdated(AIPerception)
  (params (Actor :type Actor%20Object%20Reference) (Stimulus :type AI%20Stimulus%20Structure))
  (CallFunction|UpdateEnemyKeyBlackboard Stimulus Actor Actor))

(event EventBeginPlay
  (bind _blackboardcomponent (Class|AIController|UseBlackboard "/Game/Dynamic/Character/AI/PatrolData.PatrolData"))
  (AI|RunBehaviorTree "/Game/Dynamic/Character/AI/GuardBehaviour.GuardBehaviour")
  (Variables|Default|SetBlackboardComponent _blackboardcomponent))

(fn ConstructionScript)

(fn UpdateEnemyKeyBlackboard
  (params (AIStimulus :type AI%20Stimulus%20Structure%20%28by%20ref%29) (self2 :type Actor%20Object%20Reference) (InputPin :type Actor%20Object%20Reference))
  (if (Actor|ActorHasTag self2 "Enemy")
    (AI|Components|Blackboard|SetValueasObject (Variables|Default|GetBlackboardComponent) (Variables|Default|GetEnemy%20Key) InputPin :!label _label)
    (elif (.bSuccessfullySensed (Utilities|Struct|BreakAIStimulus AIStimulus))
      (goto _label))))